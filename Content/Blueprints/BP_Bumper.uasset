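; BP_Bumper is a bumper that knocks the player character away horizontally on overlap and plays a bump animation.
; The overlap applies a velocity-change impulse to the player's capsule along the X and Y of the bumper-to-player direction, scaled by LaunchVelocity.
; A timeline adds BumpTrack to the cylinder's current scale each update, so the change accumulates, then resets it to RestingScale when finished.
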(event `self.ReceiveActorBeginOverlap`
  (params (OtherActor :type "Actor Object Reference"))
  (bind _cylinder (`self.Cylinder`))
  (bind _asbp_player_character (cast `/Game/Blueprints/BP_PlayerCharacter` (`GameplayStatics.GetPlayerCharacter` 0)))
  (if (== OtherActor _asbp_player_character)
    (bind (_returnvalue_x _returnvalue_y) (`KismetMathLibrary.BreakVector` (* (`KismetMathLibrary.GetDirectionUnitVector` (`self.K2_GetActorLocation`) (`self.K2_GetActorLocation` _asbp_player_character)) (`self.Launch Velocity`))))
    (`PrimitiveComponent.AddImpulse` (`Character.CapsuleComponent` _asbp_player_character) (`KismetMathLibrary.MakeVector` _returnvalue_x _returnvalue_y) "None" true)
    (bind (_direction _bump_track) (`Timeline|Timeline` :!via `PlayFromStart`)
      (:`Update`
        (`SceneComponent.SetRelativeScale3D` _cylinder (+ (`SceneComponent.RelativeScale3D` _cylinder) _bump_track)))
      (:`Finished`
        (`SceneComponent.SetRelativeScale3D` _cylinder (`self.Resting Scale`))))))

(fn `UserConstructionScript`)