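; Side bumper actor that knocks the player character away on overlap with velocity-change impulses scaled by LaunchVelocity.
; Three boxes push along their rotation yawed 90 degrees, while three capsules push horizontally outward from their centers.
; Actor-level overlap also adds a horizontal push away from the actor's origin.
; Box and capsule overlaps replay a shared scale-punch Timeline that resets to RestingScale, and a separate AudioBox plays the bumper sound.
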(event `self.ReceiveActorBeginOverlap`
  (params (OtherActor :type "Actor Object Reference"))
  (bind _asbp_player_character (cast `/Game/Blueprints/BP_PlayerCharacter` (`GameplayStatics.GetPlayerCharacter` 0)))
  (if (== OtherActor _asbp_player_character)
    (bind (_returnvalue_x _returnvalue_y) (`KismetMathLibrary.BreakVector` (* (`KismetMathLibrary.GetDirectionUnitVector` (`self.K2_GetActorLocation`) (`self.K2_GetActorLocation` _asbp_player_character)) (`self.Launch Velocity`))))
    (`PrimitiveComponent.AddImpulse` (`Character.CapsuleComponent` _asbp_player_character) (`KismetMathLibrary.MakeVector` _returnvalue_x _returnvalue_y) "None" true)))

(event `self.Box.OnComponentBeginOverlap`
  (params (OverlappedComponent :type "PrimitiveComponent Object Reference") (OtherActor :type "Actor Object Reference") (OtherComp :type "PrimitiveComponent Object Reference") (OtherBodyIndex :type Integer) (bFromSweep :type Boolean) (SweepResult :type "HitResult Structure (by ref)"))
  (bind _side_bumper (`self.side_bumper`))
  (`self.AddDirectionalImpulse` OverlappedComponent OtherActor)
  (bind (_direction _side_bumper_track) (`Timeline|Timeline` :!via `PlayFromStart` :!label _label)
    (:`Update`
      (`SceneComponent.SetRelativeScale3D` _side_bumper (+ (`SceneComponent.RelativeScale3D` _side_bumper) _side_bumper_track)))
    (:`Finished`
      (`SceneComponent.SetRelativeScale3D` _side_bumper (`self.Resting Scale`)))))

(event `self.Box1.OnComponentBeginOverlap`
  (params (OverlappedComponent :type "PrimitiveComponent Object Reference") (OtherActor :type "Actor Object Reference") (OtherComp :type "PrimitiveComponent Object Reference") (OtherBodyIndex :type Integer) (bFromSweep :type Boolean) (SweepResult :type "HitResult Structure (by ref)"))
  (`self.AddDirectionalImpulse` OverlappedComponent OtherActor)
  (goto _label :!via `PlayFromStart`))

(event `self.Box2.OnComponentBeginOverlap`
  (params (OverlappedComponent :type "PrimitiveComponent Object Reference") (OtherActor :type "Actor Object Reference") (OtherComp :type "PrimitiveComponent Object Reference") (OtherBodyIndex :type Integer) (bFromSweep :type Boolean) (SweepResult :type "HitResult Structure (by ref)"))
  (`self.AddDirectionalImpulse` OverlappedComponent OtherActor)
  (goto _label :!via `PlayFromStart`))

(event `self.Capsule.OnComponentBeginOverlap`
  (params (OverlappedComponent :type "PrimitiveComponent Object Reference") (OtherActor :type "Actor Object Reference") (OtherComp :type "PrimitiveComponent Object Reference") (OtherBodyIndex :type Integer) (bFromSweep :type Boolean) (SweepResult :type "HitResult Structure (by ref)"))
  (`self.CapsuleDirectionalImpulse` OverlappedComponent OtherActor)
  (goto _label :!via `PlayFromStart`))

(event `self.Capsule1.OnComponentBeginOverlap`
  (params (OverlappedComponent :type "PrimitiveComponent Object Reference") (OtherActor :type "Actor Object Reference") (OtherComp :type "PrimitiveComponent Object Reference") (OtherBodyIndex :type Integer) (bFromSweep :type Boolean) (SweepResult :type "HitResult Structure (by ref)"))
  (`self.CapsuleDirectionalImpulse` OverlappedComponent OtherActor)
  (goto _label :!via `PlayFromStart`))

(event `self.Capsule2.OnComponentBeginOverlap`
  (params (OverlappedComponent :type "PrimitiveComponent Object Reference") (OtherActor :type "Actor Object Reference") (OtherComp :type "PrimitiveComponent Object Reference") (OtherBodyIndex :type Integer) (bFromSweep :type Boolean) (SweepResult :type "HitResult Structure (by ref)"))
  (`self.CapsuleDirectionalImpulse` OverlappedComponent OtherActor)
  (goto _label :!via `PlayFromStart`))

(event `self.AudioBox.OnComponentBeginOverlap`
  (params (OverlappedComponent :type "PrimitiveComponent Object Reference") (OtherActor :type "Actor Object Reference") (OtherComp :type "PrimitiveComponent Object Reference") (OtherBodyIndex :type Integer) (bFromSweep :type Boolean) (SweepResult :type "HitResult Structure (by ref)"))
  (`GameplayStatics.PlaySoundAtLocation` "/Game/Audio/Interactable/Audio_Bumpers.Audio_Bumpers" (`self.K2_GetActorLocation`) (struct) 1.0 1.0 0.0 null null null null))

(fn `AddDirectionalImpulse`
  (params (overlapComp :type "SceneComponent Object Reference") (`other actor` :type "Object Object Reference"))
  (bind (_returnvalue_roll _returnvalue_pitch _returnvalue_yaw) (`KismetMathLibrary.BreakRotator` (`SceneComponent.K2_GetComponentRotation` overlapComp)))
  (bind (_returnvalue_x _returnvalue_y _returnvalue_z) (`KismetMathLibrary.BreakVector` (`KismetMathLibrary.MakeVector` _returnvalue_roll _returnvalue_pitch (+ _returnvalue_yaw 90.0))))
  (bind _asbp_player_character (cast `/Game/Blueprints/BP_PlayerCharacter` (`GameplayStatics.GetPlayerCharacter` 0)))
  (if (== `other actor` _asbp_player_character)
    (`PrimitiveComponent.AddImpulse` (`Character.CapsuleComponent` _asbp_player_character) (* (`KismetMathLibrary.GetForwardVector` (`KismetMathLibrary.MakeRotator` _returnvalue_x _returnvalue_y _returnvalue_z)) (`self.Launch Velocity`)) "None" true)))

(fn `CapsuleDirectionalImpulse`
  (params (self2 :type "SceneComponent Object Reference") (A :type "Object Object Reference"))
  (bind _asbp_player_character (cast `/Game/Blueprints/BP_PlayerCharacter` (`GameplayStatics.GetPlayerCharacter` 0)))
  (if (== A _asbp_player_character)
    (bind (_returnvalue_x _returnvalue_y) (`KismetMathLibrary.BreakVector` (* (`KismetMathLibrary.GetDirectionUnitVector` (`SceneComponent.K2_GetComponentLocation` self2) (`self.K2_GetActorLocation` _asbp_player_character)) (`self.Launch Velocity`))))
    (`PrimitiveComponent.AddImpulse` (`Character.CapsuleComponent` _asbp_player_character) (`KismetMathLibrary.MakeVector` _returnvalue_x _returnvalue_y) "None" true)))

(fn `UserConstructionScript`)