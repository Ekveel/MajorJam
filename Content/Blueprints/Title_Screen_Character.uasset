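; Title screen character actor that moves a static mesh along a spline in a continuous loop.
; Each tick advances the distance along the spline by a speed variable and resets it to zero past the spline's end.
; The mesh takes the spline's local location, roll and yaw, while its pitch combines spline pitch with negated travel distance, scaled by a rotation speed, to spin it as it moves.
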(event `self.ReceiveTick`
  (params (DeltaSeconds :type "Float (single-precision)"))
  (bind (_returnvalue_location _returnvalue_rotation) (`KismetMathLibrary.BreakTransform` (`SplineComponent.GetTransformAtDistanceAlongSpline` (`self.Spline`) (`self.Distance Along Spline`) "Local" false)))
  (set `self.Distance Along Spline` (+ (* DeltaSeconds (`self.Spline Speed`)) (`self.Distance Along Spline`)))
  (`SceneComponent.K2_SetRelativeTransform` (`self.StaticMesh`) (`KismetMathLibrary.MakeTransform` _returnvalue_location (`KismetMathLibrary.MakeRotator` (.roll _returnvalue_rotation) (* (+ (.pitch _returnvalue_rotation) (* (`self.Distance Along Spline`) -1.0)) (`self.Rotation Speed`)) (.yaw _returnvalue_rotation)) (`SceneComponent.RelativeScale3D` (`self.StaticMesh`))) false false)
  (if (> (`self.Distance Along Spline`) (`SplineComponent.GetSplineLength` (`self.Spline`)))
    (set `self.Distance Along Spline` 0.0)))

(fn `UserConstructionScript`)