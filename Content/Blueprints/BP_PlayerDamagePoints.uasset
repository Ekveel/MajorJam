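; BP_PlayerDamagePoints is a hazard volume that drains the player's Water while the player character is inside its box.
; Box overlap events set a flag when BP_PlayerCharacter enters and clear it when any overlap ends.
; A looping half-second timer checks the flag, subtracts BaseDamage from Water on BP_GameModeMain, then calls its DestroyPlayer on every damage tick.
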(event `self.ReceiveBeginPlay`
  ;[0 0 0] Loser Water over time
  (`KismetSystemLibrary.K2_SetTimerDelegate` (delegate `DamageTick`) 0.5 true))

(event `DamageTick`
  ;[0 0 0] Loser Water over time
  (if (`self.IsOverlapping`)
    (bind _asbp_game_mode_main (cast `/Game/Blueprints/BP_GameModeMain` (`GameplayStatics.GetGameMode`)))
    (set `/Game/Blueprints/BP_GameModeMain.Water` (- (`/Game/Blueprints/BP_GameModeMain.Water` _asbp_game_mode_main) (`self.BaseDamage`)) _asbp_game_mode_main)
    (`/Game/Blueprints/BP_GameModeMain.DestroyPlayer` _asbp_game_mode_main)))

(event `self.Box.OnComponentBeginOverlap`
  (params (OverlappedComponent :type "PrimitiveComponent Object Reference") (OtherActor :type "Actor Object Reference") (OtherComp :type "PrimitiveComponent Object Reference") (OtherBodyIndex :type Integer) (bFromSweep :type Boolean) (SweepResult :type "HitResult Structure (by ref)"))
  (bind _asbp_player_character (cast `/Game/Blueprints/BP_PlayerCharacter` OtherActor))
  (bind _output_get (set `self.PlayerCharacterRef` _asbp_player_character))
  (`/Engine/EditorBlueprintResources/StandardMacros.IsValid` _output_get
    (:`Is Valid`
      (set `self.IsOverlapping` true))))

(event `self.Box.OnComponentEndOverlap`
  (params (OverlappedComponent :type "PrimitiveComponent Object Reference") (OtherActor :type "Actor Object Reference") (OtherComp :type "PrimitiveComponent Object Reference") (OtherBodyIndex :type Integer))
  (set `self.IsOverlapping` false))

(fn `UserConstructionScript`)