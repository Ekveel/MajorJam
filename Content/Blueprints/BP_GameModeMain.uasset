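; Main game mode that creates the player HUD and handles checkpoint respawns, level loss and level completion.
; Respawning costs Water, then spawns and possesses a new character at CurrentCheckpoint, or calls DestroyPlayer if Water equals exactly zero.
; DestroyPlayer removes the character once and shows the lose screen.
; WinLevel writes level 1 completion to a fresh save object, shows the finish screen and freezes the character through disabled input and extreme damping.
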(event `self.ReceiveBeginPlay`
  (bind _returnvalue (`|CreateWidget` "/Game/UI/WBP_PlayerHUD.WBP_PlayerHUD_C"))
  (`UserWidget.AddToViewport` _returnvalue 0))

(event `DestroyPlayer`
  (bind _returnvalue (`GameplayStatics.GetPlayerController` 0))
  (if (<= (`self.Water`) 0.0)
    (`/Engine/EditorBlueprintResources/StandardMacros.DoOnce` false
      (:`Completed`
        (`self.DisableInput` (`GameplayStatics.GetPlayerCharacter` 0) _returnvalue)
        (set `PlayerController.bShowMouseCursor` true _returnvalue)
        (`self.K2_DestroyActor` (`GameplayStatics.GetPlayerCharacter` 0))
        (bind _returnvalue_2 (`|CreateWidget` "/Game/UI/WBP_LoseLevel.WBP_LoseLevel_C"))
        (`UserWidget.AddToViewport` _returnvalue_2 0)))))

(event `WinLevel`
  (bind _returnvalue (`GameplayStatics.GetPlayerCharacter` 0))
  (bind _returnvalue_2 (`GameplayStatics.GetPlayerController` 0))
  (bind _capsulecomponent (`Character.CapsuleComponent` _returnvalue))
  (bind _returnvalue_3 (`GameplayStatics.CreateSaveGameObject` "/Game/Blueprints/BP_SaveGame.BP_SaveGame_C"))
  (set `/Game/Blueprints/BP_SaveGame.FinishedLvl1` true _returnvalue_3)
  (`GameplayStatics.SaveGameToSlot` _returnvalue_3 "Slot1")
  (bind _returnvalue_4 (`|CreateWidget` "/Game/UI/WBP_FinishLevel.WBP_FinishLevel_C"))
  (`UserWidget.AddToViewport` _returnvalue_4 0)
  (`self.DisableInput` _returnvalue _returnvalue_2)
  (set `PlayerController.bShowMouseCursor` true _returnvalue_2)
  (`PrimitiveComponent.SetLinearDamping` _capsulecomponent 999999999999999.0)
  (`PrimitiveComponent.SetAngularDamping` _capsulecomponent 999999999999999.0))

(event `RespawnPlayer`
  (bind _output_get (set `self.OldWaterLevel` (`self.Water`)))
  (bind _output_get_2 (set `self.Water` (- _output_get 10.0)))
  (if (== _output_get_2 0.0)
    (`self.DestroyPlayer`)
    (else
      (bind _returnvalue (`|SpawnActorFromClass` "/Game/Blueprints/BP_PlayerCharacter.BP_PlayerCharacter_C" (`self.CurrentCheckpoint`) "Undefined" "MultiplyWithRoot" null null))
      (`self.K2_DestroyActor` (`GameplayStatics.GetPlayerCharacter` 0))
      (`Controller.Possess` (`GameplayStatics.GetPlayerController` 0) _returnvalue)
      (`/Game/Blueprints/BP_PlayerCharacter.Speed` _returnvalue (`/Game/Blueprints/BP_PlayerCharacter.PlayerSpeed` _returnvalue)))))

(fn `UserConstructionScript`)